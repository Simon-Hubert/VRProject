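; Game mode for a VR space level that starts play under normal gravity, then switches to zero gravity after a short timer.
; On BeginPlay it finds the start room gravity manager and VR pawn, initializes the GravityWorldSubsystem and sets Earth-like global gravity.
; When the timer fires, it zeroes global gravity through the subsystem and has the room manager impulse physics actors.
; EndGame is an empty stub.
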(event Custom|CE_DeactivateGravity
  (bind _startroomgravitymanager (Variables|Default|GetStartRoomGravityManager))
  (Class|GravityWorldSubsystem|SetGlobalGravityZ (Subsystems|GetGravityWorldSubsystem) 0.0)
  (Utilities|IsValid _startroomgravitymanager
    (:Is%20Valid
      (Default|ImpulsePhysicsActor _startroomgravitymanager))
    (:Is%20Not%20Valid
      (Development|PrintString "Start Room Manager Not Valid. Can't Impulse." true true "(R=1.000000,G=0.113890,B=0.127259,A=1.000000)"))))

(event EventBeginPlay
  (CallFunction|InitGame)
  (CallFunction|StartGame)
  (Utilities|Time|SetTimerbyEvent (delegate Custom|CE_DeactivateGravity) 1e+01))

(fn ConstructionScript)

(fn InitGame
  (Utilities|FlowControl|Sequence
    (:then_0
      (bind _returnvalue (Actor|GetActorOfClass "/Game/_Project/Blueprints/Gravity/BP_StartRoomGravityManager.BP_StartRoomGravityManager_C"))
      (Utilities|IsValid _returnvalue
        (:Is%20Valid
          (Variables|Default|SetStartRoomGravityManager _returnvalue)
          (Development|PrintString "SpaceGM: Found Start Room Gravity Manager" true true "(R=0.137371,G=1.000000,B=0.204610,A=1.000000)"))
        (:Is%20Not%20Valid
          (Development|PrintString "SpaceGM: Didn't find Start Room Gravity Manager" true true "(R=1.000000,G=0.113890,B=0.127259,A=1.000000)"))))
    (:then_1
      (bind _returnvalue_2 (Actor|GetActorOfClass "/Game/_Project/Blueprints/VRCharacter/BP_VRPawn.BP_VRPawn_C"))
      (Utilities|IsValid _returnvalue_2
        (:Is%20Valid
          (Variables|Default|SetPlayer _returnvalue_2)
          (Development|PrintString "SpaceGM: Found Player" true true "(R=0.137371,G=1.000000,B=0.204610,A=1.000000)"))
        (:Is%20Not%20Valid
          (Development|PrintString "SpaceGM: Didn't find Player" true true "(R=1.000000,G=0.113890,B=0.127259,A=1.000000)"))))
    (:then_2
      (Class|GravityWorldSubsystem|InitGravityWorldSubsystem (Subsystems|GetGravityWorldSubsystem)))))

(fn StartGame
  (Class|GravityWorldSubsystem|SetGlobalGravityZ (Subsystems|GetGravityWorldSubsystem) -981.0))

(fn EndGame)