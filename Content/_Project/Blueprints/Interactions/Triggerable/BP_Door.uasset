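; BP_Door is a triggerable double sliding door that alternates between opening and closing each time it is triggered with the matching interaction type.
; A FlipFlop in OnTrigger picks the open or close event, which plays or reverses the OpenDoor timeline to slide the left and right meshes apart or together along X.
; Both events play the door sound through the BP_SoundManager found at BeginPlay.
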(event Custom|CE_Open
  (bind _returnvalue (Math|Float|MakeLiteralFloat 1e+02))
  (Default|Door (Variables|Default|GetSoundManager))
  (bind _p (Timeline|OpenDoor Play)
    (:Update
      (Transformation|SetRelativeLocation (Variables|Default|GetSM_DoorRight) (Math|Vector|MakeVector (* _returnvalue _p) 0.0 0.0) false false)
      (Transformation|SetRelativeLocation (Variables|Default|GetSM_DoorLeft) (Math|Vector|MakeVector (- 0.0 (* _returnvalue _p)) 0.0 0.0) false false))))

(event Custom|CE_Close
  (bind _returnvalue (Math|Float|MakeLiteralFloat 1e+02))
  (Default|Door (Variables|Default|GetSoundManager))
  (bind _p (Timeline|OpenDoor ReverseFromEnd)
    (:Update
      (Transformation|SetRelativeLocation (Variables|Default|GetSM_DoorRight) (Math|Vector|MakeVector (* _returnvalue _p) 0.0 0.0) false false)
      (Transformation|SetRelativeLocation (Variables|Default|GetSM_DoorLeft) (Math|Vector|MakeVector (- 0.0 (* _returnvalue _p)) 0.0 0.0) false false))))

(event EventBeginPlay
  (bind _returnvalue (Actor|GetActorOfClass "/Game/_Project/Blueprints/SoundManager/BP_SoundManager.BP_SoundManager_C"))
  (Variables|Default|SetSoundManager _returnvalue))

(event EventOnTrigger
  (params (InteractionType :type E_InteractionType%20Enum :default "NewEnumerator0"))
  (Development|PrintString "try open door")
  (if (Utilities|Enum|Equal(Enum) InteractionType "NewEnumerator0")
    (Development|PrintString "open door")
    (Utilities|FlowControl|FlipFlop
      (:A
        (CallFunction|CEOpen))
      (:B
        (CallFunction|CEClose)))))

(fn ConstructionScript)