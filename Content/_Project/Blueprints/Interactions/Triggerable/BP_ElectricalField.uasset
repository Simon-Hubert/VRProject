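; BP_ElectricalField is a triggerable hazard that periodically switches between lethal and harmless, killing damageable actors inside it.
; Overlap events maintain a list of BPI_Damageable actors, while a looping timer with an initial delay flip-flops the damage state.
; While active and damaging, Tick calls Kill on the list in reverse, removing successful kills safely.
; OnTrigger with the first interaction type deactivates the field, with no reactivation path.
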(event Custom|CE_ToggleElectricity
  (Utilities|FlowControl|FlipFlop
    (:A
      (CallFunction|CEActivateDamages))
    (:B
      (CallFunction|CEDeActivateDamages))))

(event Custom|CE_ActivateDamages
  (Variables|Default|SetDoesDamages true))

(event Custom|CE_DeactivateDamages
  (Variables|Default|SetDoesDamages false))

(event Collision|EventActorBeginOverlap
  (params (OtherActor :type Actor%20Object%20Reference))
  (bind _asbpi_damageable (Utilities|Casting|CastToBPI_Damageable OtherActor))
  (Utilities|Array|Add (Variables|Default|GetToDamage) _asbpi_damageable))

(event Collision|EventActorEndOverlap
  (params (OtherActor :type Actor%20Object%20Reference))
  (bind _todamage (Variables|Default|GetToDamage))
  (bind _asbpi_damageable (Utilities|Casting|CastToBPI_Damageable OtherActor))
  (if (Utilities|Array|ContainsItem _todamage _asbpi_damageable)
    (Utilities|Array|RemoveItem _todamage _asbpi_damageable)))

(event EventBeginPlay
  (Utilities|Time|SetTimerbyEvent (delegate Custom|CE_ToggleElectricity) (Variables|Default|GetDuration) true true (Variables|Default|GetInitialDelay)))

(event EventOnTrigger
  (params (InteractionType :type E_InteractionType%20Enum :default "NewEnumerator0"))
  (if (Utilities|Enum|Equal(Enum) InteractionType "NewEnumerator0")
    (Variables|Default|SetIsActive false)))

(event EventTick
  (params (DeltaSeconds :type Float%20%28single-precision%29))
  (if (Variables|Default|GetIsActive)
    (if (Variables|Default|GetDoesDamages)
      (bind (_arrayindex _arrayelement) (Utilities|Array|ReverseforEachLoop (Variables|Default|GetToDamage))
        (:LoopBody
          (bind _killed (Default|Kill _arrayelement))
          (if _killed
            (Utilities|Array|RemoveIndex (Variables|Default|GetToDamage) _arrayindex)))))))

(fn ConstructionScript)