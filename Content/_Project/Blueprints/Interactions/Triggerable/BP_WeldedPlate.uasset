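; BP_WeldedPlate is a triggerable plate held in place by a set of weldings until all of them are undone.
; It binds to each welding's unweld event at BeginPlay and rechecks the whole set whenever one fires.
; Once all are undone, it opens, adds a grab component to the plate, enables physics and broadcasts OnUnwelded.
; Triggers of one interaction type then run its interact event and broadcast OnInteracted.
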(event Custom|OnUnwelding_Event
  (bind _result (CallFunction|AreAllWeldingsUndone))
  (if _result
    (CallFunction|CEAllWeldingsUndone)))

(event Custom|CE_AllWeldingsUndone
  (bind _plate (Variables|Default|GetPlate))
  (Variables|Default|SetIsOpen true)
  (bind _returnvalue (AddComponent|AddBPGrabComponent false))
  (Transformation|AttachComponentToComponent _returnvalue _plate "None" "KeepRelative" "KeepRelative" "KeepRelative" true)
  (Physics|SetSimulatePhysics _plate true)
  (Default|CallOnUnwelded))

(event EventBeginPlay
  (for _array_element (Variables|Default|GetWeldings)
    (EventDispatchers|AssignOnUnwelding _array_element (delegate Custom|OnUnwelding_Event))))

(event EventOnTrigger
  (params (InteractionType :type E_InteractionType%20Enum :default "NewEnumerator0"))
  (if (and (Utilities|Enum|Equal(Enum) InteractionType "NewEnumerator2") (Variables|Default|GetIsOpen))
    (CallFunction|CEInteract "NewEnumerator0")
    (Default|CallOnInteracted)))

(fn ConstructionScript)

(fn AreAllWeldingsUndone
  (for _array_element (Variables|Default|GetWeldings)
    (if (not (Variables|/Game/_Project/Blueprints/Interactions/Triggerable/BP_Welding.BP_Welding_C|GetIsUnwelded _array_element))
      (return false)))
  (return true))