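; BP_EngineerTool is a grabbable VR multi-tool that cycles through Burner, Screw Driver and Discharge modes on the right-hand main button.
; Its sphere overlap finds BPI_Triggerable actors: Burner interacts on overlap while firing, while the other modes track targets and interact on trigger.
; Changing mode clears targets and burning.
; When inputs are active, grabbing adds the holding hand's weapon mapping context and hides its hand message; dropping reverses this.
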(event OnComponentBeginOverlap(Sphere)
  (params (OverlappedComponent :type Primitive%20Component%20Object%20Reference) (OtherActor :type Actor%20Object%20Reference) (OtherComp :type Primitive%20Component%20Object%20Reference) (OtherBodyIndex :type Integer) (bFromSweep :type Boolean) (SweepResult :type Hit%20Result%20Structure%20%28by%20ref%29))
  (bind _targets (Variables|Default|GetTargets))
  (switch Utilities|FlowControl|Switch|SwitchonE_ToolState (Variables|Default|GetCurrent%20State)
    (:NewEnumerator0
      (bind _asbpi_triggerable (Utilities|Casting|CastToBPI_Triggerable OtherActor))
      (if (Variables|Default|GetIsBurning)
        (Utilities|Array|Add _targets _asbpi_triggerable)
        (CallFunction|CEInteract "NewEnumerator1")
        (Utilities|Array|RemoveItem _targets _asbpi_triggerable)))
    (:NewEnumerator1
      (bind _asbpi_triggerable_2 (Utilities|Casting|CastToBPI_Triggerable OtherActor :!label _label))
      (Utilities|Array|Add (Variables|Default|GetTargets) _asbpi_triggerable_2))
    (:NewEnumerator2
      (goto _label))))

(event OnComponentEndOverlap(Sphere)
  (params (OverlappedComponent :type Primitive%20Component%20Object%20Reference) (OtherActor :type Actor%20Object%20Reference) (OtherComp :type Primitive%20Component%20Object%20Reference) (OtherBodyIndex :type Integer))
  (bind _targets (Variables|Default|GetTargets))
  (switch Utilities|FlowControl|Switch|SwitchonE_ToolState (Variables|Default|GetCurrent%20State)
    (:NewEnumerator1
      _)
    (:NewEnumerator2
      _))
  (bind _asbpi_triggerable (Utilities|Casting|CastToBPI_Triggerable OtherActor))
  (if (Utilities|Array|ContainsItem _targets _asbpi_triggerable)
    (Utilities|Array|RemoveItem _targets _asbpi_triggerable)))

(event OnGrabbed(GrabComponent)
  (params (MotionController :type Motion%20Controller%20Component%20Object%20Reference) (ActorGrabbed :type Actor%20Object%20Reference))
  (bind _grabcomponent (Variables|Default|GetGrabComponent))
  (bind _returnvalue (Default|GetHeldbyHand _grabcomponent))
  (bind _returnvalue_2 (Utilities|Enum|Equal(Enum) _returnvalue "Right"))
  (if (Variables|Default|GetAreInputActive)
    (Input|EnableInput (Game|GetPlayerController 0))
    (Class|BPIPawnAnim|HideUnhideHand(Message) (Components|GetOwner (Variables|/Game/_Project/Blueprints/Grabbable/BP_GrabComponent.BP_GrabComponent_C|GetMotionControllerRef _grabcomponent)) true _returnvalue_2)
    (Input|AddMappingContext (PlayerController|LocalPlayerSubsystems|GetEnhancedInputLocalPlayerSubsystem (Game|GetPlayerController 0)) (select _returnvalue_2 "/Game/VRTemplate/Input/IMC_Weapon_Right.IMC_Weapon_Right" "/Game/VRTemplate/Input/IMC_Weapon_Left.IMC_Weapon_Left") 1 "(bIgnoreAllPressedKeysUntilRelease=True,bForceImmediately=False,bNotifyUserSettings=False)")
    (Default|CallOnGrabbed)))

(event OnDropped(GrabComponent)
  (params (ActorDropped :type Actor%20Object%20Reference))
  (bind _grabcomponent (Variables|Default|GetGrabComponent))
  (bind _returnvalue (Default|GetHeldbyHand _grabcomponent))
  (bind _returnvalue_2 (Utilities|Enum|Equal(Enum) _returnvalue "Right"))
  (Input|DisableInput (Game|GetPlayerController 0))
  (Class|BPIPawnAnim|HideUnhideHand(Message) (Components|GetOwner (Variables|/Game/_Project/Blueprints/Grabbable/BP_GrabComponent.BP_GrabComponent_C|GetMotionControllerRef _grabcomponent)) false _returnvalue_2)
  (Input|RemoveMappingContext (PlayerController|LocalPlayerSubsystems|GetEnhancedInputLocalPlayerSubsystem (Game|GetPlayerController 0)) (select _returnvalue_2 "/Game/VRTemplate/Input/IMC_Weapon_Right.IMC_Weapon_Right" "/Game/VRTemplate/Input/IMC_Weapon_Left.IMC_Weapon_Left") "(bIgnoreAllPressedKeysUntilRelease=True,bForceImmediately=False,bNotifyUserSettings=False)")
  (Default|CallOnDropped))

(event Custom|CE_EnableInputs
  (bind _grabcomponent (Variables|Default|GetGrabComponent))
  (bind _returnvalue (Default|GetHeldbyHand _grabcomponent))
  (bind _returnvalue_2 (Utilities|Enum|Equal(Enum) _returnvalue "Right"))
  (Variables|Default|SetAreInputActive true)
  (if (Variables|/Game/_Project/Blueprints/Grabbable/BP_GrabComponent.BP_GrabComponent_C|GetbIsHeld (Variables|Default|GetGrabComponent))
    (Input|EnableInput (Game|GetPlayerController 0))
    (Class|BPIPawnAnim|HideUnhideHand(Message) (Components|GetOwner (Variables|/Game/_Project/Blueprints/Grabbable/BP_GrabComponent.BP_GrabComponent_C|GetMotionControllerRef _grabcomponent)) true _returnvalue_2)
    (Input|AddMappingContext (PlayerController|LocalPlayerSubsystems|GetEnhancedInputLocalPlayerSubsystem (Game|GetPlayerController 0)) (select _returnvalue_2 "/Game/VRTemplate/Input/IMC_Weapon_Right.IMC_Weapon_Right" "/Game/VRTemplate/Input/IMC_Weapon_Left.IMC_Weapon_Left") 1 "(bIgnoreAllPressedKeysUntilRelease=True,bForceImmediately=False,bNotifyUserSettings=False)")
    (Default|CallOnGrabbed)))

(event Input|EnhancedActionEvents|EnhancedInputActionIA_Shoot_Right
  (params (ActionValue :type Boolean) (ElapsedSeconds :type Float%20%28double-precision%29) (TriggeredSeconds :type Float%20%28double-precision%29) (InputAction :type Input%20Action%20Object%20Reference :default "/Game/VRTemplate/Input/Actions/IA_Shoot_Right.IA_Shoot_Right"))
  (:Triggered
    (if (Utilities|Enum|Equal(Enum) (Default|GetHeldbyHand (Variables|Default|GetGrabComponent)) "Right")
      (switch Utilities|FlowControl|Switch|SwitchonE_ToolState (Variables|Default|GetCurrent%20State)
        (:NewEnumerator0
          (Variables|Default|SetIsBurning true))
        (:NewEnumerator1
          (CallFunction|CEInteract "NewEnumerator3"))
        (:NewEnumerator2
          (CallFunction|CEInteract "NewEnumerator2")))))
  (:Canceled
    (if (Utilities|Enum|Equal(Enum) (Default|GetHeldbyHand (Variables|Default|GetGrabComponent)) "Right")
      (switch Utilities|FlowControl|Switch|SwitchonE_ToolState (Variables|Default|GetCurrent%20State)
        (:NewEnumerator0
          (Variables|Default|SetIsBurning false))))))

(event Input|EnhancedActionEvents|EnhancedInputActionIA_Shoot_Left
  (params (ActionValue :type Boolean) (ElapsedSeconds :type Float%20%28double-precision%29) (TriggeredSeconds :type Float%20%28double-precision%29) (InputAction :type Input%20Action%20Object%20Reference :default "/Game/VRTemplate/Input/Actions/IA_Shoot_Left.IA_Shoot_Left"))
  (:Triggered
    (if (Utilities|Enum|Equal(Enum) (Default|GetHeldbyHand (Variables|Default|GetGrabComponent)) "Left")
      (switch Utilities|FlowControl|Switch|SwitchonE_ToolState (Variables|Default|GetCurrent%20State)
        (:NewEnumerator0
          (Variables|Default|SetIsBurning true))
        (:NewEnumerator1
          (CallFunction|CEInteract "NewEnumerator3"))
        (:NewEnumerator2
          (CallFunction|CEInteract "NewEnumerator2")))))
  (:Canceled
    (if (Utilities|Enum|Equal(Enum) (Default|GetHeldbyHand (Variables|Default|GetGrabComponent)) "Left")
      (switch Utilities|FlowControl|Switch|SwitchonE_ToolState (Variables|Default|GetCurrent%20State)
        (:NewEnumerator0
          (Variables|Default|SetIsBurning false))))))

(event Input|EnhancedActionEvents|EnhancedInputActionIA_Hand_MainButton_Right
  (params (ActionValue :type Boolean) (ElapsedSeconds :type Float%20%28double-precision%29) (TriggeredSeconds :type Float%20%28double-precision%29) (InputAction :type Input%20Action%20Object%20Reference :default "/Game/_Project/Assets/Inputs/IA_Hand_MainButton_Right.IA_Hand_MainButton_Right"))
  (:Started
    (if (Variables|/Game/_Project/Blueprints/Grabbable/BP_GrabComponent.BP_GrabComponent_C|GetbIsHeld (Variables|Default|GetGrabComponent))
      (switch Utilities|FlowControl|Switch|SwitchonE_ToolState (Variables|Default|GetCurrent%20State)
        (:NewEnumerator0
          (CallFunction|ChangeState "NewEnumerator1"))
        (:NewEnumerator1
          (CallFunction|ChangeState "NewEnumerator2"))
        (:NewEnumerator2
          (CallFunction|ChangeState "NewEnumerator0")))
      (Development|PrintString (Utilities|String|Append "Current State : " (Utilities|String|EnumtoString (Variables|Default|GetCurrent%20State)))))))

(event EventBeginPlay
  (Default|CEDischarge (Variables|Default|GetBP_DischargeVFX)))

(fn ConstructionScript
  (|CallParentFunction))

(fn ChangeState
  (params (NewState :type E_ToolState%20Enum :default "NewEnumerator0"))
  (Variables|Default|SetCurrent%20State NewState)
  (CallFunction|Reset))

(fn Reset
  (Utilities|Array|Clear (Variables|Default|GetTargets))
  (Variables|Default|SetIsBurning false))