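; Rope actor that visually links a Player to a Hold through a cable component.
; Init stores the Player and attaches the cable end to it, while a separate event swaps the current Hold.
; Each tick moves the actor to the location the Hold returns for the Player's position.
; The construction script sets cable length from Length, scaled by 100 as if converting meters to centimeters.
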(event Custom|CE_Init
  (params (Player :type BP%20VR%20Pawn%20Object%20Reference))
  (bind _output_get (Variables|Default|SetPlayer Player))
  (Class|CableComponent|SetAttachEndto (Variables|Default|GetRope) _output_get "None" "None"))

(event Custom|CE_UpdateHold
  (params (NewHold :type BP%20Hold%20Base%20Object%20Reference))
  (Variables|Default|SetHold NewHold))

(event EventTick
  (params (DeltaSeconds :type Float%20%28single-precision%29))
  (bind _location (Default|GetLocation (Variables|Default|GetHold) (.location (Transformation|GetActorTransform (Variables|Default|GetPlayer)))))
  (Transformation|SetActorLocation _location false false))

(fn ConstructionScript
  (Variables|/Script/CableComponent.CableComponent|SetCableLength (Variables|Default|GetRope) (* (Variables|Default|GetLength) 1e+02)))