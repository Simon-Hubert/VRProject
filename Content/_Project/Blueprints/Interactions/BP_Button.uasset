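; BP_Button is an interactable push button that a BP_VRPawn triggers by overlapping its Collision component.
; Begin overlap prints a debug "Hello", calls CEInteract, fires OnPressed and runs the pressed animation event.
; End overlap runs the released animation event, with no other notification.
; Both animation events instantly set the Button component's relative Z location, with no interpolation.
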(event OnComponentBeginOverlap(Collision)
  (params (OverlappedComponent :type Primitive%20Component%20Object%20Reference) (OtherActor :type Actor%20Object%20Reference) (OtherComp :type Primitive%20Component%20Object%20Reference) (OtherBodyIndex :type Integer) (bFromSweep :type Boolean) (SweepResult :type Hit%20Result%20Structure%20%28by%20ref%29))
  (Utilities|Casting|CastToBP_VRPawn OtherActor)
  (Development|PrintString "Hello")
  (CallFunction|CEInteract "NewEnumerator0")
  (Default|CallOnPressed)
  (CallFunction|CEAnimPressed))

(event OnComponentEndOverlap(Collision)
  (params (OverlappedComponent :type Primitive%20Component%20Object%20Reference) (OtherActor :type Actor%20Object%20Reference) (OtherComp :type Primitive%20Component%20Object%20Reference) (OtherBodyIndex :type Integer))
  (Utilities|Casting|CastToBP_VRPawn OtherActor)
  (CallFunction|CEAnimReleased))

(event Custom|CE_AnimReleased
  (Transformation|SetRelativeLocation (Variables|Default|GetButton) (Math|Vector|MakeVector 0.0 0.0 15.0) false false))

(event Custom|CE_AnimPressed
  (Transformation|SetRelativeLocation (Variables|Default|GetButton) (Math|Vector|MakeVector 0.0 0.0 5.0) false false))

(fn ConstructionScript
  (|CallParentFunction))