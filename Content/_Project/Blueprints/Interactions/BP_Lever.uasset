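; BP_Lever is a grabbable VR lever that fires an interact event when pulled past a trigger percentage.
; While grabbed, Tick converts the motion controller's location into the Ref component's local space and uses atan2 to pitch the Pivot, clamped between MinAngle and MaxAngle.
; The pivot's angle is normalized across that range, and crossing TriggerPercent calls CEInteract through a DoOnce that is never reset.
; The construction script starts the Pivot at MinAngle.
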(event OnGrabbed(BP_GrabComponent)
  (params (MotionController :type Motion%20Controller%20Component%20Object%20Reference) (ActorGrabbed :type Actor%20Object%20Reference))
  (Variables|Default|SetMotion%20Controller MotionController))

(event OnDropped(BP_GrabComponent)
  (params (ActorDropped :type Actor%20Object%20Reference))
  (Variables|Default|SetMotion%20Controller 0))

(event EventTick
  (params (DeltaSeconds :type Float%20%28single-precision%29))
  (bind _pivot (Variables|Default|GetPivot))
  (bind _returnvalue (Math|Vector|GetUpVector _pivot))
  (bind _motion_controller (Variables|Default|GetMotion%20Controller)
    (:then
      (Transformation|SetRelativeRotation (Variables|Default|GetPivot) (Math|Rotator|MakeRotator 0.0 (Math|Float|Clamp(Float) (Class|KismetMathLibrary|DegAtan2 (.z (Math|Transform|InverseTransformLocation (Transformation|GetWorldTransform (Variables|Default|GetRef)) (Transformation|GetWorldLocation _motion_controller))) (.x (Math|Transform|InverseTransformLocation (Transformation|GetWorldTransform (Variables|Default|GetRef)) (Transformation|GetWorldLocation _motion_controller)))) (Variables|Default|GetMinAngle) (Variables|Default|GetMaxAngle)) 0.0) false false)
      (if (> (|((T-A)/(B-A)) (- 0.0 (Class|KismetMathLibrary|DegAtan2 (.x _returnvalue) (.z _returnvalue))) (Variables|Default|GetMinAngle) (Variables|Default|GetMaxAngle)) (Variables|Default|GetTriggerPercent))
        (Utilities|FlowControl|DoOnce false
          (:Completed
            (CallFunction|CEInteract)))))
    (:else)))

(fn ConstructionScript
  (|CallParentFunction)
  (Transformation|SetRelativeRotation (Variables|Default|GetPivot) (Math|Rotator|MakeRotator 0.0 (Variables|Default|GetMinAngle) 0.0) false false))