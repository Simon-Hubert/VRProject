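; Scene component that renders an electrical field effect between two splines attached to it as children.
; On BeginPlay it stores the first two child spline components and runs only if both are found.
; Tick throttles spawning by Rate per second, each time creating a pooled NS_ElectricField Niagara system.
; Each system gets StartPoint and EndPoint parameters from random world-space points along the first and second spline.
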(event Custom|CE_SpawnSystem
  (bind (_start _end) (CallFunction|GetRandomPointsonSplines))
  (bind _returnvalue (Niagara|SpawnSystemAttached "/Game/_Project/Assets/Art/VFX/NS_ElectricField.NS_ElectricField" self "None" "0, 0, 0" "0, 0, 0" "KeepWorldPosition" true true "AutoRelease"))
  (Effects|Components|ParticleSystem|SetVectorParameter _returnvalue "StartPoint" _start)
  (Effects|Components|ParticleSystem|SetVectorParameter _returnvalue "EndPoint" _end))

(event EventBeginPlay
  (bind _array_element (Utilities|Array|ForEachLoopwithBreak (Components|GetChildrenComponents false) :!label _label)
    (:LoopBody
      (bind _asspline_component (Utilities|Casting|CastToSplineComponent _array_element))
      (if (Utilities|IsValid (Variables|Default|GetSpline1))
        (if (not (Utilities|IsValid (Variables|Default|GetSpline2)))
          (Variables|Default|SetSpline2 _asspline_component)
          (goto _label Break))
        (else
          (Variables|Default|SetSpline1 _asspline_component))))
    (:Completed
      (Variables|Default|SetIsCorrectlyInit (and (Utilities|IsValid (Variables|Default|GetSpline1)) (Utilities|IsValid (Variables|Default|GetSpline2)))))))

(event EventTick
  (params (DeltaSeconds :type Float%20%28single-precision%29))
  (bind _returnvalue (Utilities|Time|GetTimeSeconds))
  (if (Variables|Default|GetIsCorrectlyInit)
    (if (>= (- _returnvalue (Variables|Default|GetLastProc)) (/ 1.0 (Variables|Default|GetRate)))
      (Variables|Default|SetLastProc _returnvalue)
      (CallFunction|CESpawnSystem))))

(fn GetRandomPointsonSplines
  (bind _spline1 (Variables|Default|GetSpline1))
  (bind _spline2 (Variables|Default|GetSpline2))
  (return (Spline|GetLocationatDistanceAlongSpline _spline1 (* (Spline|GetSplineLength _spline1) (Math|Random|RandomFloat)) "World") (Spline|GetLocationatDistanceAlongSpline _spline2 (* (Spline|GetSplineLength _spline2) (Math|Random|RandomFloat)) "World")))