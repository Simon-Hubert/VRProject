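; BP_DischargeVFX is a component that plays an electric discharge effect when its CE_Discharge event fires.
; It spawns a configurable number of pooled, attached Niagara arcs, each running from a random point in a cone around its right vector to the component's location.
; A single attached burst system, rotated relative to the component, completes the effect.
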(event Custom|CE_Discharge
  (bind _returnvalue (Transformation|GetWorldLocation))
  (for _index (range 0 (Variables|Default|GetNumber))
    (bind _returnvalue_2 (Niagara|SpawnSystemAttached "/Game/_Project/Assets/Art/VFX/NS_ElectricDischarge.NS_ElectricDischarge" self "None" "0, 0, 0" "0, 0, 0" "KeepWorldPosition" true true "AutoRelease"))
    (Effects|Components|ParticleSystem|SetVectorParameter _returnvalue_2 "EndPoint" _returnvalue)
    (Effects|Components|ParticleSystem|SetVectorParameter _returnvalue_2 "StartPoint" (+ _returnvalue (* (Math|Random|RandomUnitVectorinConeinDegrees (Math|Vector|GetRightVector) (Variables|Default|GetConeHalfAngle)) 25.0))))
  (Niagara|SpawnSystemAttached "/Game/_Project/Assets/Art/VFX/NS_Burst.NS_Burst" self "None" "0, 0, 0" "0.000000,90.000000,0.000000" "KeepRelativeOffset" true true "AutoRelease"))