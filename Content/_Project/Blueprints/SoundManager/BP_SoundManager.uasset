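; BP_SoundManager is a sound manager that plays music, looping breathing, air-conditioner and intro dialogue as 2D sounds.
; StartMusic spawns and stores the music component, then a timeline lerps its volume from the starting level to a fixed target.
; The breath-in and breath-out events call each other on fixed delays to form an endless loop.
; BeginPlay is empty and the chains that sequence these events are disconnected, so nothing starts by itself.
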(event EventBeginPlay)

(event EventPlayDialogueIntro
  (Audio|PlaySound2D "/Game/_Project/Blueprints/SoundManager/Sound/Dialogue_Intro.Dialogue_Intro" 1.0 1.0 0.0 0 0))

(event EventStartMusic
  ;[0.15 0.15 0.15 0.5] Play Music
  (bind _returnvalue (Audio|SpawnSound2D (Variables|Music|GetMusic) (Variables|Music|GetVolumeMusic) 1.0 0.0 0))
  (Variables|Default|SetMusique _returnvalue)
  ;;[0.15 0.15 0.15 0.5] Set le volume petit a petit
  (bind _newtrack_0 (Timeline|SetVolumMusic PlayFromStart)
    (:Update
      (Audio|Components|Audio|SetVolumeMultiplier (Variables|Default|GetMusique) (Math|Float|Lerp (Variables|Music|GetVolumeMusic) 0.6 _newtrack_0) :!class /Script/Engine.AudioComponent))))

(event EventBreathOut
  ;[0.15 0.15 0.15 0.5] Play Breath
  (Audio|PlaySound2D "/Game/_Project/Blueprints/SoundManager/Sound/SC_Breath_Out.SC_Breath_Out" 0.2 1.0 0.0 0 0)
  (Utilities|FlowControl|Delay 4.0)
  (CallFunction|Breathin))

(event EventBreathin
  ;[0.15 0.15 0.15 0.5] Play Breath
  (Audio|PlaySound2D "/Game/_Project/Blueprints/SoundManager/Sound/SC_Breath_In.SC_Breath_In" 0.2 1.0 0.0 0 0)
  (Utilities|FlowControl|Delay 4.0)
  (CallFunction|BreathOut))

(event EventPlayAir
  ;[0.07842 0.03197 0.15 0.5] Play Air
  (Audio|PlaySound2D "/Game/_Project/Blueprints/SoundManager/Sound/Inside_aircondisioner.Inside_aircondisioner" 1.0 1.0 0.0 0 0)
  (Development|PrintString "Play Air" true true "(R=0.137371,G=1.000000,B=0.204610,A=1.000000)"))

(fn ConstructionScript)