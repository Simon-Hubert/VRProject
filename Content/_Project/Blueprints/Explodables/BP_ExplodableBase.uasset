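; BP_ExplodableBase is an explodable actor, named as a base class, that pushes its surroundings with a radial impulse and then disappears.
; The construction script applies ExplosionRadius to both the Sphere and RadialForce components and sets the impulse strength from ExplosionStrenght.
; The Explode event prints a debug message, fires the RadialForce impulse and destroys the actor; nothing in these graphs calls it.
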(event EventExplode
  (Development|PrintString "Explosion" true true "(R=1.000000,G=0.591804,B=0.198477,A=1.000000)")
  (Class|RadialForceComponent|FireImpulse (Variables|Default|GetRadialForce))
  (Actor|DestroyActor))

(fn ConstructionScript
  (bind _explosionradius (Variables|Explosion|GetExplosionRadius))
  (Components|Sphere|SetSphereRadius (Variables|Default|GetSphere) _explosionradius false)
  (Variables|/Script/Engine.RadialForceComponent|SetRadius (Variables|Default|GetRadialForce) _explosionradius)
  (Variables|/Script/Engine.RadialForceComponent|SetImpulseStrength (Variables|Default|GetRadialForce) (Variables|Explosion|GetExplosionStrenght)))