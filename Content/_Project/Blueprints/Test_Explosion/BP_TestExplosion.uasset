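; Test trigger actor that sets off a station explosion when the VR pawn enters its box.
; On BeginPlay it finds the Geometry Collection and master field actors, freezes the collection's physics and gravity, and creates a player for the Station_Explodes sequence.
; The overlap plays the sequence, waits briefly, then re-enables physics and fires the field's CETrigger to break the collection.
; TestEvent enters the same chain without an overlap.
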(event OnComponentBeginOverlap(Box)
  (params (OverlappedComponent :type Primitive%20Component%20Object%20Reference) (OtherActor :type Actor%20Object%20Reference) (OtherComp :type Primitive%20Component%20Object%20Reference) (OtherBodyIndex :type Integer) (bFromSweep :type Boolean) (SweepResult :type Hit%20Result%20Structure%20%28by%20ref%29))
  (bind _gc (Variables|Default|GetGC))
  (Utilities|Casting|CastToBP_VRPawn OtherActor)
  (Sequencer|Player|Play (Variables|Default|GetAnimation) :!class /Script/MovieScene.MovieSceneSequencePlayer)
  (Utilities|FlowControl|Delay 2.4)
  (Physics|SetEnableGravity (Variables|/Game/_Project/Assets/Art/Meshes/Chaos/BP_GC.BP_GC_C|GetGeometryCollection _gc) true)
  (Physics|SetSimulatePhysics (Variables|/Game/_Project/Assets/Art/Meshes/Chaos/BP_GC.BP_GC_C|GetGeometryCollection _gc) true)
  (Default|CETrigger (Variables|Default|GetMaster_Field)))

(event Custom|TestExplosion)

(event Custom|TestEvent
  (bind _gc (Variables|Default|GetGC))
  (Sequencer|Player|Play (Variables|Default|GetAnimation) :!class /Script/MovieScene.MovieSceneSequencePlayer)
  (Utilities|FlowControl|Delay 2.4)
  (Physics|SetEnableGravity (Variables|/Game/_Project/Assets/Art/Meshes/Chaos/BP_GC.BP_GC_C|GetGeometryCollection _gc) true)
  (Physics|SetSimulatePhysics (Variables|/Game/_Project/Assets/Art/Meshes/Chaos/BP_GC.BP_GC_C|GetGeometryCollection _gc) true)
  (Default|CETrigger (Variables|Default|GetMaster_Field)))

(event EventBeginPlay
  (bind _returnvalue (Actor|GetActorOfClass "/Game/_Project/Assets/Art/Meshes/Chaos/BP_GC.BP_GC_C"))
  (bind _output_get (Variables|Default|SetGC _returnvalue))
  (Physics|SetEnableGravity (Variables|/Game/_Project/Assets/Art/Meshes/Chaos/BP_GC.BP_GC_C|GetGeometryCollection _output_get) false)
  (Physics|SetSimulatePhysics (Variables|/Game/_Project/Assets/Art/Meshes/Chaos/BP_GC.BP_GC_C|GetGeometryCollection _output_get) false)
  (bind _returnvalue_2 (Sequencer|Player|CreateLevelSequencePlayer "/Game/_Project/Assets/Art/Sequences/Station_Explodes.Station_Explodes"))
  (Variables|Default|SetAnimation _returnvalue_2)
  (bind _returnvalue_3 (Actor|GetActorOfClass "/Game/_Project/Assets/Art/Meshes/Chaos/FS_MasterField.FS_MasterField_C"))
  (Variables|Default|SetMaster_Field _returnvalue_3)
  (Development|PrintString "Tout trouvé")
  (Utilities|FlowControl|Delay 3.0))

(fn ConstructionScript)