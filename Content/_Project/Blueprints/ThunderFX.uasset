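; Actor component that surrounds its owner with lightning effects that strike nearby surfaces, plus an attached effect spawned on BeginPlay.
; On a cooldown checked each Tick, it attempts two bolts, tracing between inner and outer radii along random downward-hemisphere vectors, scaled shorter toward straight down.
; Each blocking hit spawns an attached particle system, fed start point, end point and impact normal as parameters.
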(event EventBeginPlay
  (Niagara|SpawnSystemAttached 0 (Variables|/Script/Engine.Actor|GetRootComponent (Components|GetOwner)) "None" "0.000000,0.000000,50.000000" "0, 0, 0" "KeepRelativeOffset" false))

(event EventTick
  (params (DeltaSeconds :type Float%20%28single-precision%29))
  (CallFunction|Update))

(fn Update
  (if (>= (- (Utilities|Time|GetTimeSeconds) (Variables|Default|GetLastProc)) (Variables|Default|GetCooldown))
    (Variables|Default|SetLastProc (Utilities|Time|GetTimeSeconds))
    (CallFunction|TrySpawnBolt)
    (CallFunction|TrySpawnBolt)))

(fn TrySpawnBolt
  (bind _returnvalue (Components|GetOwner))
  (bind _returnvalue_2 (Math|Float|MultiplybyPi 0.5))
  (bind _returnvalue_3 (Class|KismetMathLibrary|RandomUnitVectorinConeinRadians "0.000000,0.000000,-1.000000" _returnvalue_2))
  (bind _returnvalue_4 (Transformation|GetActorLocation _returnvalue))
  ;[1 1 1] LineTrace
  (LocalVariables|SetRndVector (Math|Vector|ClampVectorSize (* _returnvalue_3 (+ (- 1.0 (Math|Vector|DotProduct _returnvalue_3 "0.000000,0.000000,-1.000000")) 0.0)) 0.0 1.0))
  (bind _outhit (Collision|LineTraceByChannel (+ (* (LocalVariables|GetRndVector) (Variables|Default|GetMinRadius)) _returnvalue_4) (+ _returnvalue_4 (* (LocalVariables|GetRndVector) (Variables|Default|GetMaxRadius))) "TraceTypeQuery1" false 0 "None" true "(R=1.000000,G=0.000000,B=0.000000,A=1.000000)" "(R=0.000000,G=1.000000,B=0.000000,A=1.000000)" 1.0))
  ;[1 1 1] Spawn System
  (if (.bblockinghit _outhit)
    (bind _returnvalue_5 (Niagara|SpawnSystemAttached 0 (Variables|/Script/Engine.Actor|GetRootComponent (Components|GetOwner)) "None" "0, 0, 0" "0, 0, 0" "KeepRelativeOffset" false))
    (Effects|Components|ParticleSystem|SetVectorParameter _returnvalue_5 "StartPoint" (* (LocalVariables|GetRndVector) (Variables|Default|GetMinRadius)))
    (Effects|Components|ParticleSystem|SetVectorParameter _returnvalue_5 "EndPoint" (+ (.location _outhit) (* (.normal _outhit) 1.0)))
    (Effects|Components|ParticleSystem|SetVectorParameter _returnvalue_5 "ImpactNormal" (.normal _outhit))))