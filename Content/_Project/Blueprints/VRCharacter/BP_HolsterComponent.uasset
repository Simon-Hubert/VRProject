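; BP_HolsterComponent is a VR character holster that keeps the dropped engineer tool at the component's location.
; On BeginPlay it finds a BP_EngineerTool in the level, caches its Visual and binds to its dropped and grabbed events.
; Those events toggle a flag, and while it is set Tick moves the Visual to the holster's world location, leaving rotation untouched.
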(event Custom|CE_OnToolDropped
  (Variables|Default|SetIsToolDropped true))

(event Custom|CE_OnToolGrabbed
  (Variables|Default|SetIsToolDropped false))

(event EventBeginPlay
  (bind _returnvalue (Actor|GetActorOfClass "/Game/_Project/Blueprints/Interactions/BP_EngineerTool.BP_EngineerTool_C"))
  (Utilities|IsValid _returnvalue
    (:Is%20Valid
      (Variables|Default|SetVisual (Variables|/Game/_Project/Blueprints/Interactions/BP_EngineerTool.BP_EngineerTool_C|GetVisual _returnvalue))
      (EventDispatchers|BindEventtoOnDropped _returnvalue (delegate Custom|CE_OnToolDropped))
      (EventDispatchers|BindEventtoOnGrabbed _returnvalue (delegate Custom|CE_OnToolGrabbed)))))

(event EventTick
  (params (DeltaSeconds :type Float%20%28single-precision%29))
  (if (Variables|Default|GetIsToolDropped)
    (bind _visual (Variables|Default|GetVisual)
      (:then
        (Transformation|SetWorldLocation _visual (Transformation|GetWorldLocation) false false))
      (:else))))