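; BP_Holster is a VR holster actor that follows the player and holds the engineer tool when it is not in hand.
; On begin play it finds the VR pawn's camera and the engineer tool, binding to the tool's grabbed and dropped events.
; Each tick it moves to the camera's world location plus a fixed offset, unrotated, and snaps a dropped tool onto its root until grabbed again.
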(event Custom|CE_OnToolDropped
  (Variables|Default|SetIsToolDropped true))

(event Custom|CE_OnToolGrabbed
  (Variables|Default|SetIsToolDropped false))

(event EventBeginPlay
  (Utilities|FlowControl|Sequence
    (:then_0
      (bind _returnvalue (Actor|GetActorOfClass "/Game/_Project/Blueprints/VRCharacter/BP_VRPawn.BP_VRPawn_C"))
      (Utilities|IsValid _returnvalue
        (:Is%20Valid
          (Variables|Default|SetCamera (Variables|/Game/_Project/Blueprints/VRCharacter/BP_VRPawn.BP_VRPawn_C|GetCamera _returnvalue)))))
    (:then_1
      (bind _returnvalue_2 (Actor|GetActorOfClass "/Game/_Project/Blueprints/Interactions/BP_EngineerTool.BP_EngineerTool_C"))
      (Utilities|IsValid _returnvalue_2
        (:Is%20Valid
          (bind _output_get (Variables|Default|SetTool _returnvalue_2))
          (EventDispatchers|BindEventtoOnDropped _output_get (delegate Custom|CE_OnToolDropped))
          (EventDispatchers|BindEventtoOnGrabbed _output_get (delegate Custom|CE_OnToolGrabbed)))))))

(event EventTick
  (params (DeltaSeconds :type Float%20%28single-precision%29))
  (bind _camera (Variables|Default|GetCamera)
    (:then
      (Transformation|SetActorLocation (+ (Transformation|GetWorldLocation _camera) (Variables|Default|GetOffset)) false false)
      (if (Variables|Default|GetIsToolDropped)
        (bind _tool (Variables|Default|GetTool)
          (:then
            (Transformation|SetActorLocation _tool (Transformation|GetWorldLocation (Variables|Default|GetDefaultSceneRoot)) false false))
          (:else))))
    (:else)))

(fn ConstructionScript)