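; Health component that tracks an actor's current health, starting at MaxHealth on BeginPlay.
; TakeDamage ignores dead owners, subtracts clamped damage with debug prints, and calls the Died dispatcher when IsDead reports death.
; Heal and Kill appear to have inverted checks: Heal only applies at or above max health, and Kill only calls TakeDamage when already dead.
; IsDead's health comparison is left unconnected.
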(event EventBeginPlay
  (Variables|Health|SetCurrentHealth (Variables|Health|GetMaxHealth)))

(fn Heal
  (params (Heal :type Float%20%28double-precision%29))
  (if (>= (Variables|Health|GetCurrentHealth) (Variables|Health|GetMaxHealth))
    (Variables|Health|SetCurrentHealth (Math|Float|Clamp(Float) (+ (Variables|Health|GetCurrentHealth) Heal) 0.0 (Variables|Health|GetMaxHealth)))
    (return true)
    (else
      (return false))))

(fn Kill
  (if (Utilities|IsDead)
    (CallFunction|TakeDamage (+ (Variables|Health|GetMaxHealth) 1.0))
    (return true)
    (else
      (return false))))

(fn TakeDamage
  (params (Damage :type Float%20%28double-precision%29))
  (if (Utilities|IsDead)
    (return false)
    (else
      (Development|PrintString "Took Damage" true true "(R=1.000000,G=0.591804,B=0.198477,A=1.000000)")
      (Variables|Health|SetCurrentHealth (Math|Float|Clamp(Float) (- (Variables|Health|GetCurrentHealth) Damage) 0.0 (Variables|Health|GetMaxHealth)))
      (if (Utilities|IsDead)
        (Development|PrintString "Died From Damage" true true "(R=1.000000,G=0.591804,B=0.198477,A=1.000000)")
        (Default|CallDied)
        (return true)
        (else
          (return true))))))