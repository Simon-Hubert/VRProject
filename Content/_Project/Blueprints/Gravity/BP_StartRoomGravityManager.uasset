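; Gravity manager for the start room that turns a gravity button press into a one-time GravityDeactivated dispatcher call.
; A DoOnce on the button's OnPressed event guards against repeat broadcasts.
; A separate ImpulsePhysicsActor function, not called within this Blueprint, applies a shared impulse to the primitive root of each listed physics actor, with debug prints for the call and failed casts.
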(event OnPressed(GravityButton)
  (Utilities|FlowControl|DoOnce false
    (:Completed
      (Default|CallGravityDeactivated))))

(fn ConstructionScript)

(fn ImpulsePhysicsActor
  (Development|PrintString "Impulse Physics Actors" true true "(R=0.756866,G=0.116645,B=1.000000,A=1.000000)")
  (for _array_element (Variables|StartRoomGravityManager|GetPhysicsActorToImpulse)
    (bind _asprimitive_component (Utilities|Casting|CastToPrimitiveComponent (Variables|/Script/Engine.Actor|GetRootComponent _array_element))
      (:then
        (Physics|AddImpulse _asprimitive_component (Variables|StartRoomGravityManager|GetImpulseForce) "None" false))
      (:CastFailed
        (Development|PrintString "Actor Impulse Failed: Root is not a Primitive Component" true true "(R=1.000000,G=0.113890,B=0.127259,A=1.000000)"))))
  (return))